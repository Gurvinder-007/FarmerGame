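; BP_House is a shop building that opens the WB_Shop menu when the player's pawn enters its Box trigger.
; The overlap creates and caches the widget on first use, passes it a back-reference to the house, then shows it with UI-only input and mouse cursor.
; A SpawnActor event spawns any given class at a given transform, adjusting for collisions but always spawning.
; Closing the menu is not handled here.
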(event OnComponentEndOverlap(StaticMesh)
  (params (OverlappedComponent :type Primitive%20Component%20Object%20Reference) (OtherActor :type Actor%20Object%20Reference) (OtherComp :type Primitive%20Component%20Object%20Reference) (OtherBodyIndex :type Integer)))

(event OnComponentBeginOverlap(Box)
  (params (OverlappedComponent :type Primitive%20Component%20Object%20Reference) (OtherActor :type Actor%20Object%20Reference) (OtherComp :type Primitive%20Component%20Object%20Reference) (OtherBodyIndex :type Integer) (bFromSweep :type Boolean) (SweepResult :type Hit%20Result%20Structure%20%28by%20ref%29))
  (bind _returnvalue (Game|GetPlayerController 0))
  (if (== (Pawn|GetControlledPawn (Game|GetPlayerController 0)) OtherActor)
    (Utilities|IsValid (Variables|Default|GetWB_Shop)
      (:Is%20Valid
        _)
      (:Is%20Not%20Valid
        (bind _returnvalue_2 (UserInterface|CreateWidget "/Game/Shop/WB_Shop.WB_Shop_C"))
        (bind _output_get (Variables|Default|SetWB_Shop _returnvalue_2))
        (Variables|/Game/Shop/WB_Shop.WB_Shop_C|SetBP_Shop _output_get self)))
    (if (not (UserInterface|Viewport|IsinViewport (Variables|Default|GetWB_Shop)))
      (UserInterface|Viewport|AddtoViewport (Variables|Default|GetWB_Shop) 0)
      (Input|SetInputModeUIOnly _returnvalue 0 "DoNotLock" false)
      (Variables|/Script/Engine.PlayerController|SetbShowMouseCursor _returnvalue true))))

(event Custom|Spawn%20Actor
  (params (Class :type Actor%20Class%20Reference) (SpawnTransform :type Transform))
  (Game|SpawnActorfromClass Class SpawnTransform "AdjustIfPossibleButAlwaysSpawn" "MultiplyWithRoot" 0 0))

(event EventBeginPlay)

(event EventTick
  (params (DeltaSeconds :type Float%20%28single-precision%29)))

(fn ConstructionScript)