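; BP_FarmTile is a farm plot actor where the player plants and harvests wheat, corn or pumpkin.
; PlantSeed follows the character's selected seed, checking stock for wheat and corn but not pumpkin, then swaps three growth meshes between GrowTime countdowns shown on Text3D.
; Activate calls Harvest, which clears grown crops and credits every type to AmountOfWheat; loose-item spawns key off WhatCanBeHarvested, only ever set empty here.
; Overlapping the FarmTile component destroys the actor.
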(event OnComponentBeginOverlap(FarmTile)
  (params (OverlappedComponent :type Primitive%20Component%20Object%20Reference) (OtherActor :type Actor%20Object%20Reference) (OtherComp :type Primitive%20Component%20Object%20Reference) (OtherBodyIndex :type Integer) (bFromSweep :type Boolean) (SweepResult :type Hit%20Result%20Structure%20%28by%20ref%29))
  (Actor|DestroyActor))

(event Custom|PlantWheat
  (bind _relativetransformlocation (Variables|Default|GetRelativeTransformLocation))
  (bind _returnvalue (AddComponent|AddStaticMeshComponent false (Math|Transform|MakeTransform _relativetransformlocation "0, 0, 0" "1.000000,1.000000,1.000000")))
  (Utilities|GrowTime (Variables|Default|GetWheatGrowTime)
    (:Out
      (Components|DestroyComponent _returnvalue)
      (bind _returnvalue_2 (AddComponent|AddStaticMeshComponent false (Math|Transform|MakeTransform _relativetransformlocation "0, 0, 0" "1.000000,1.000000,1.000000")))
      (Utilities|GrowTime (Variables|Default|GetWheatGrowTime)
        (:Out
          (Components|DestroyComponent _returnvalue_2)
          (bind _returnvalue_3 (AddComponent|AddStaticMeshComponent false (Math|Transform|MakeTransform _relativetransformlocation "0, 0, 0" "1.000000,1.000000,1.000000")))
          (Variables|Default|SetFullyGrown? true)
          (Variables|Default|SetCurrentMesh _returnvalue_3)
          (Variables|Default|SetWhatCanBeHarvested ""))))))

(event Custom|PlantPumpkin
  (bind _relativetransformlocation (Variables|Default|GetRelativeTransformLocation))
  (bind _returnvalue (AddComponent|AddStaticMeshComponent false (Math|Transform|MakeTransform _relativetransformlocation "0, 0, 0" "1.000000,1.000000,1.000000")))
  (Utilities|GrowTime (Variables|Default|GetWheatGrowTime)
    (:Out
      (Components|DestroyComponent _returnvalue)
      (bind _returnvalue_2 (AddComponent|AddStaticMeshComponent false (Math|Transform|MakeTransform _relativetransformlocation "0, 0, 0" "1.000000,1.000000,1.000000")))
      (Utilities|GrowTime (Variables|Default|GetWheatGrowTime)
        (:Out
          (Components|DestroyComponent _returnvalue_2)
          (bind _returnvalue_3 (AddComponent|AddStaticMeshComponent false (Math|Transform|MakeTransform _relativetransformlocation "0, 0, 0" "1.000000,1.000000,1.000000")))
          (Variables|Default|SetFullyGrown? true)
          (Variables|Default|SetCurrentMesh _returnvalue_3)
          (Variables|Default|SetWhatCanBeHarvested ""))))))

(event Custom|PlantCorn
  (bind _relativetransformlocation (Variables|Default|GetRelativeTransformLocation))
  (bind _returnvalue (AddComponent|AddStaticMeshComponent false (Math|Transform|MakeTransform _relativetransformlocation "0, 0, 0" "1.000000,1.000000,1.000000")))
  (Utilities|GrowTime (Variables|Default|GetWheatGrowTime)
    (:Out
      (Components|DestroyComponent _returnvalue)
      (bind _returnvalue_2 (AddComponent|AddStaticMeshComponent false (Math|Transform|MakeTransform _relativetransformlocation "0, 0, 0" "1.000000,1.000000,1.000000")))
      (Utilities|GrowTime (Variables|Default|GetWheatGrowTime)
        (:Out
          (Components|DestroyComponent _returnvalue_2)
          (bind _returnvalue_3 (AddComponent|AddStaticMeshComponent false (Math|Transform|MakeTransform _relativetransformlocation "0, 0, 0" "1.000000,1.000000,1.000000")))
          (Variables|Default|SetFullyGrown? true)
          (Variables|Default|SetCurrentMesh _returnvalue_3)
          (Variables|Default|SetWhatCanBeHarvested ""))))))

(event EventPlantSeed
  (if (not (Variables|Default|GetIsSomethingPlanted?))
    (bind _asbp_third_person_character (Utilities|Casting|CastToBP_ThirdPersonCharacter (Game|GetPlayerCharacter 0)))
    (switch int (Variables|/Game/ThirdPerson/Blueprints/BP_ThirdPersonCharacter.BP_ThirdPersonCharacter_C|GetSeed _asbp_third_person_character)
      (:0
        (Utilities|DoWeHaveWheatSeed
          (:Output
            (CallFunction|PlantWheat)
            (Variables|Default|SetIsWheat? true))))
      (:1
        (Utilities|DoWeHaveCornSeed
          (:Output
            (CallFunction|PlantCorn)
            (Variables|Default|SetIsCorn? true))))
      (:2
        (CallFunction|PlantPumpkin)
        (Variables|Default|SetIsPumpkin? true)))
    (Variables|Default|SetIsSomethingPlanted? true)))

(event EventBeginPlay
  (Class|Text3DComponent|SetText (Variables|Default|GetText3D) (Variables|Default|GetValue)))

(event EventActivate
  (CallFunction|Harvest))

(fn ConstructionScript)

(fn Harvest
  (bind _text3d (Variables|Default|GetText3D))
  (bind _text3d_2 (Variables|Default|GetText3D))
  (bind _text3d_3 (Variables|Default|GetText3D))
  (bind _returnvalue (Transformation|GetWorldLocation _text3d_3))
  (bind _returnvalue_2 (Transformation|GetWorldLocation _text3d_2))
  (bind _returnvalue_3 (Transformation|GetWorldLocation _text3d))
  (bind _returnvalue_4 (Math|Conversions|ToTransform(Vector) _returnvalue_2))
  (bind _returnvalue_5 (Math|Conversions|ToTransform(Vector) _returnvalue))
  (bind _returnvalue_6 (Math|Conversions|ToTransform(Vector) _returnvalue_3))
  (if (Variables|Default|GetFullyGrown?)
    (if (Variables|Default|GetIsWheat?)
      (Components|DestroyComponent (Variables|Default|GetCurrentMesh))
      (bind _asbp_third_person_character (Utilities|Casting|CastToBP_ThirdPersonCharacter (Game|GetPlayerCharacter 0)))
      (bind _result (Math|Integer|IncrementInt (Variables|/Game/ThirdPerson/Blueprints/BP_ThirdPersonCharacter.BP_ThirdPersonCharacter_C|GetAmountOfWheat _asbp_third_person_character))
        (:%20%20
          (Variables|/Game/ThirdPerson/Blueprints/BP_ThirdPersonCharacter.BP_ThirdPersonCharacter_C|SetAmountOfWheat _asbp_third_person_character _result)
          ;[1 1 1] Check for bugs
          (switch string (Variables|Default|GetWhatCanBeHarvested)
            (:Default
              _)
            (:Wheat
              (Default|SpawnActor (LocalVariables|GetNewLocalVar) "/Game/Blueprints/BP_WheatLoose.BP_WheatLoose_C" _returnvalue_6))
            (:Corn
              (Game|SpawnActorfromClass "/Game/Blueprints/BP_CornLoose.BP_CornLoose_C" _returnvalue_6 "Undefined" "MultiplyWithRoot" 0 0))
            (:Pumpkin
              (Game|SpawnActorfromClass "/Game/Blueprints/BP_PumpkinLoose.BP_PumpkinLoose_C" _returnvalue_6 "Undefined" "MultiplyWithRoot" 0 0)))
          (Variables|Default|SetFullyGrown? false)
          (Variables|Default|SetCurrentMesh 0)
          (Variables|Default|SetIsSomethingPlanted? false)
          (Variables|Default|SetWhatCanBeHarvested "")
          (Variables|Default|SetIsWheat? false)))
      (elif (Variables|Default|GetIsCorn?)
        (Components|DestroyComponent (Variables|Default|GetCurrentMesh))
        (bind _asbp_third_person_character_2 (Utilities|Casting|CastToBP_ThirdPersonCharacter (Game|GetPlayerCharacter 0)))
        (bind _result_2 (Math|Integer|IncrementInt (+ 1 (Variables|/Game/ThirdPerson/Blueprints/BP_ThirdPersonCharacter.BP_ThirdPersonCharacter_C|GetAmountOfWheat _asbp_third_person_character_2)))
          (:%20%20
            (Variables|/Game/ThirdPerson/Blueprints/BP_ThirdPersonCharacter.BP_ThirdPersonCharacter_C|SetAmountOfWheat _asbp_third_person_character_2 _result_2)
            ;[1 1 1] Check for bugs
            (switch string (Variables|Default|GetWhatCanBeHarvested)
              (:Default
                _)
              (:Wheat
                (Default|SpawnActor (LocalVariables|GetNewLocalVar) "/Game/Blueprints/BP_WheatLoose.BP_WheatLoose_C" _returnvalue_4))
              (:Corn
                (Game|SpawnActorfromClass "/Game/Blueprints/BP_CornLoose.BP_CornLoose_C" _returnvalue_4 "Undefined" "MultiplyWithRoot" 0 0))
              (:Pumpkin
                (Game|SpawnActorfromClass "/Game/Blueprints/BP_PumpkinLoose.BP_PumpkinLoose_C" _returnvalue_4 "Undefined" "MultiplyWithRoot" 0 0)))
            (Variables|Default|SetFullyGrown? false)
            (Variables|Default|SetCurrentMesh 0)
            (Variables|Default|SetIsSomethingPlanted? false)
            (Variables|Default|SetWhatCanBeHarvested "")
            (Variables|Default|SetIsCorn? false)))
        (elif (Variables|Default|GetIsPumpkin?)
          (Components|DestroyComponent (Variables|Default|GetCurrentMesh))
          (bind _asbp_third_person_character_3 (Utilities|Casting|CastToBP_ThirdPersonCharacter (Game|GetPlayerCharacter 0)))
          (bind _result_3 (Math|Integer|IncrementInt (+ (Variables|/Game/ThirdPerson/Blueprints/BP_ThirdPersonCharacter.BP_ThirdPersonCharacter_C|GetAmountOfWheat _asbp_third_person_character_3) 2))
            (:%20%20
              (Variables|/Game/ThirdPerson/Blueprints/BP_ThirdPersonCharacter.BP_ThirdPersonCharacter_C|SetAmountOfWheat _asbp_third_person_character_3 _result_3)
              ;[1 1 1] Check for bugs
              (switch string (Variables|Default|GetWhatCanBeHarvested)
                (:Default
                  _)
                (:Wheat
                  (Default|SpawnActor (LocalVariables|GetNewLocalVar) "/Game/Blueprints/BP_WheatLoose.BP_WheatLoose_C" _returnvalue_5))
                (:Corn
                  (Game|SpawnActorfromClass "/Game/Blueprints/BP_CornLoose.BP_CornLoose_C" _returnvalue_5 "Undefined" "MultiplyWithRoot" 0 0))
                (:Pumpkin
                  (Game|SpawnActorfromClass "/Game/Blueprints/BP_PumpkinLoose.BP_PumpkinLoose_C" _returnvalue_5 "Undefined" "MultiplyWithRoot" 0 0)))
              (Variables|Default|SetFullyGrown? false)
              (Variables|Default|SetCurrentMesh 0)
              (Variables|Default|SetIsSomethingPlanted? false)
              (Variables|Default|SetWhatCanBeHarvested "")
              (Variables|Default|SetIsPumpkin? false))))))))

(fn PickUpItem
  (return ""))