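; BP_Item is a pickup actor that gives the player a shovel.
; PickUpItem prints a debug message, calls the AddShovel and DestroyItem events, then returns the Item value to its caller.
; AddShovel casts player 0's character to BP_ThirdPersonCharacter and sets its IsShovelInInventory flag.
; DestroyItem destroys the actor after a short delay, which runs in the event graph so the function returns first.
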(event Custom|Destroy%20Item
  (Utilities|FlowControl|Delay 0.1)
  (Actor|DestroyActor))

(event Custom|Add%20Shovel
  (bind _asbp_third_person_character (Utilities|Casting|CastToBP_ThirdPersonCharacter (Game|GetPlayerCharacter 0)))
  (Variables|/Game/ThirdPerson/Blueprints/BP_ThirdPersonCharacter.BP_ThirdPersonCharacter_C|SetisShovelInInventory? _asbp_third_person_character true))

(fn ConstructionScript)

(fn PickUpItem
  (Development|PrintString "Item Picked")
  (CallFunction|AddShovel)
  (CallFunction|DestroyItem)
  (return (Variables|Default|GetItem)))